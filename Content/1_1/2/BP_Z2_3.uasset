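; BP_Z2_3 is an actor that reports a height-based score on screen when another actor overlaps it.
; On overlap it subtracts its own Z from player 0's character Z, each converted to a 64-bit integer, and prints the difference as points in a Russian message.
; The overlapping actor is never checked, and the score is only printed, not stored.
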(event `self.ReceiveActorBeginOverlap`
  (params (OtherActor :type "Actor Object Reference"))
  (`KismetSystemLibrary.PrintString` (`KismetStringLibrary.Concat_StrStr` "Вы получили :" (`KismetStringLibrary.Conv_Int64ToString` (- (`KismetMathLibrary.Conv_DoubleToInt64` (.z (`self.K2_GetActorLocation` (`GameplayStatics.GetPlayerCharacter` 0)))) (`KismetMathLibrary.Conv_DoubleToInt64` (.z (`self.K2_GetActorLocation`))))) " очков")))

(fn `UserConstructionScript`)